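; Main menu player Blueprint that turns the view with the mouse and selects BP_InteractiveBase objects by looking at them.
; Each tick, TimeBasedGaze line-traces from the camera; a newly focused object starts a timer to Interact and spawns a BP_Timer above the hit point if none exists.
; Interact activates the object and destroys that actor, while losing focus cancels both.
; An instant-activation BasicGaze variant exists but is not called.
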(event EventTick
  (params (DeltaSeconds :type Float%20%28single-precision%29))
  (CallFunction|TimeBasedGaze))

(event Input|MouseEvents|MouseX
  (params (AxisValue :type Float%20%28single-precision%29))
  ;[1 1 1] Movimiento de la camera
  (Pawn|Input|AddControllerYawInput (* (* AxisValue (Utilities|Time|GetWorldDeltaSeconds)) (Variables|Default|GetHeadMoveSpped))))

(event Input|MouseEvents|MouseY
  (params (AxisValue :type Float%20%28single-precision%29))
  ;[1 1 1] Movimiento de la camera
  (Pawn|Input|AddControllerPitchInput (* (* AxisValue (Utilities|Time|GetWorldDeltaSeconds)) (* (Variables|Default|GetHeadMoveSpped) -1.0))))

(fn ConstructionScript)

(fn LineTrace
  (bind _camera (Variables|Default|GetCamera))
  (bind _returnvalue (Transformation|GetWorldLocation _camera))
  (bind _outhit (Collision|LineTraceByChannel _returnvalue (+ _returnvalue (* (Math|Vector|GetForwardVector (Transformation|GetWorldRotation _camera)) 1.5e+04)) "TraceTypeQuery1" false 0 "ForDuration"))
  (return _outhit))

(fn BasicGaze
  (bind _outhit (CallFunction|LineTrace))
  (bind (_bblockinghit _binitialoverlap _time _distance _location _impactpoint _normal _impactnormal _physmat _hitactor) (Collision|BreakHitResult _outhit))
  (if _bblockinghit
    (bind _asbp_interactive_base (Utilities|Casting|CastToBP_InteractiveBase _hitactor)
      (:then
        (Variables|Default|SetInteractiveObject _asbp_interactive_base)
        (if (not (== (Variables|Default|GetInteractiveObject) (Variables|Default|GetFocusedObject)))
          (Variables|Default|SetFocusedObject (Variables|Default|GetInteractiveObject))
          (CallFunction|Interact)))
      (:CastFailed
        (Variables|Default|SetFocusedObject 0 :!label _label)))
    (else
      (Variables|Default|SetInteractiveObject 0)
      (goto _label))))

(fn Interact
  (bind _interactiveobject (Variables|Default|GetInteractiveObject))
  (bind _timer_ref (Variables|Default|GetTimer%20Ref))
  (Utilities|IsValid _interactiveobject
    (:Is%20Valid
      (Default|Activate _interactiveobject)
      (Utilities|IsValid _timer_ref
        (:Is%20Valid
          (Actor|DestroyActor _timer_ref))))))

(fn TimeBasedGaze
  (bind _outhit (CallFunction|LineTrace))
  (bind (_bblockinghit _binitialoverlap _time _distance _location _impactpoint _normal _impactnormal _physmat _hitactor) (Collision|BreakHitResult _outhit))
  (if _bblockinghit
    (bind _asbp_interactive_base (Utilities|Casting|CastToBP_InteractiveBase _hitactor)
      (:then
        (Variables|Default|SetInteractiveObject _asbp_interactive_base)
        (if (not (== (Variables|Default|GetInteractiveObject) (Variables|Default|GetFocusedObject)))
          (Variables|Default|SetFocusedObject (Variables|Default|GetInteractiveObject))
          (Utilities|Time|ClearandInvalidateTimerbyHandle (Variables|Default|GetFocusTimer))
          (bind _returnvalue (Utilities|Time|SetTimerbyFunctionName 0 "Interact" (Variables|Default|GetTimer%20Lenght)))
          (Variables|Default|SetFocusTimer _returnvalue)
          (Utilities|IsValid (Variables|Default|GetTimer%20Ref)
            (:Is%20Not%20Valid
              (bind _returnvalue_2 (Game|SpawnActorfromClass "/Game/gus/Menu_Player/BP_Timer.BP_Timer_C" (Math|Transform|MakeTransform (+ _impactpoint "0, 0,50.000000") "0, 0, 0" "1,1,1") "Undefined" 0 0))
              (Variables|Default|SetTimer%20Ref _returnvalue_2)))))
      (:CastFailed
        (Variables|Default|SetFocusedObject 0 :!label _label)
        (Utilities|Time|ClearandInvalidateTimerbyHandle (Variables|Default|GetFocusTimer))
        (Utilities|IsValid (Variables|Default|GetTimer%20Ref)
          (:Is%20Valid
            (Actor|DestroyActor (Variables|Default|GetTimer%20Ref))))))
    (else
      (Variables|Default|SetInteractiveObject 0)
      (goto _label))))