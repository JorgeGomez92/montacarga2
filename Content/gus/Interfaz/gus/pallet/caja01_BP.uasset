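; Forklift cargo box that detects when it is placed on a platform and updates the player's placed-box count.
; A per-tick downward trace checks for a nearby platform, with paired DoOnce nodes toggling its traffic light and the count.
; While hit by forks and secured, the box copies their linear velocity to ride steadily.
; It also flags fork-bottom overlaps, jolts the forklift back on rack hits, and spins a pointer.
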(event OnComponentHit(StaticMeshComponent)
  (params (HitComponent :type Primitive%20Component%20Object%20Reference) (OtherActor :type Actor%20Object%20Reference) (OtherComp :type Primitive%20Component%20Object%20Reference) (NormalImpulse :type Vector :default "0, 0, 0") (Hit :type Hit%20Result%20Structure%20%28by%20ref%29))
  ;[1 1 1] si las palas chocan con algun actor con la etoqueta anaquel, reducira la fuerza del choque
  (Utilities|FlowControl|Sequence
    (:then_0
      (bind _asplataforma (Utilities|Casting|CastToplataforma OtherActor))
      (if (Utilities|Enum|Equal(Enum) (Utilities|String|ToString(Text) (Utilities|Text|ToText(Name) (Utilities|Array|Get(acopy) (Variables|/Script/Engine.ActorComponent|GetComponentTags OtherComp)))) "anaquel")
        (if (not (Class|PrimitiveComponent|IsOverlappingComponent (Variables|/Game/gus/environment/plataforma.plataforma_C|Getdetector%20palas _asplataforma) (Variables|Debug|GetStaticMeshComponent)))
          (bind _asv_3_3 (Utilities|Casting|CastTov3_3 (Game|Player|GetPlayerPawn 0)))
          (Default|TironHaciaAtras _asv_3_3))))
    (:then_1
      (if (and (not (<= (Input|AxisValues|GetMoveForward) 0.0)) (Utilities|Enum|Equal(Enum) (Utilities|String|ToString(Text) (Utilities|Text|ToText(Name) (Utilities|Array|Get(acopy) (Variables|/Script/Engine.ActorComponent|GetComponentTags OtherComp)))) "base_caja"))
        _))
    (:then_2
      (if (Utilities|Enum|Equal(Enum) (Utilities|String|ToString(Text) (Utilities|Text|ToText(Name) (Utilities|Array|Get(acopy) (Variables|/Script/Engine.Actor|GetTags OtherActor)))) "palas")
        (Variables|Default|SetgolpeaPalas true)
        (else
          (Variables|Default|SetgolpeaPalas false))))))

(event OnComponentBeginOverlap(overlapFondo)
  (params (OverlappedComponent :type Primitive%20Component%20Object%20Reference) (OtherActor :type Actor%20Object%20Reference) (OtherComp :type Primitive%20Component%20Object%20Reference) (OtherBodyIndex :type Integer) (bFromSweep :type Boolean) (SweepResult :type Hit%20Result%20Structure%20%28by%20ref%29))
  (bind _returnvalue (Utilities|GetObjectName OtherComp))
  ;[1 1 1] condicion tocar el fondo de la caja
  (bind _aspalas (Utilities|Casting|CastTopalas OtherActor))
  (if (or (Utilities|Enum|Equal(Enum) _returnvalue "palas_izq") (Utilities|Enum|Equal(Enum) _returnvalue "palas_der"))
    (Utilities|FlowControl|DoOnce false
      (:Completed
        (Variables|/Game/gus/Monta/blueprints/v3_3/palas.palas_C|Setoverlap%20fondo _aspalas true)
        (Utilities|FlowControl|DoOnce false) ; enters at Reset
      ))))

(event OnComponentEndOverlap(overlapFondo)
  (params (OverlappedComponent :type Primitive%20Component%20Object%20Reference) (OtherActor :type Actor%20Object%20Reference) (OtherComp :type Primitive%20Component%20Object%20Reference) (OtherBodyIndex :type Integer))
  (bind _returnvalue (Utilities|GetObjectName OtherComp))
  ;[1 1 1] condicion tocar el fondo de la caja
  (bind _aspalas (Utilities|Casting|CastTopalas OtherActor))
  (if (or (Utilities|Enum|Equal(Enum) _returnvalue "palas_izq") (Utilities|Enum|Equal(Enum) _returnvalue "palas_der"))
    (Utilities|FlowControl|DoOnce false
      (:Completed
        (Variables|/Game/gus/Monta/blueprints/v3_3/palas.palas_C|Setoverlap%20fondo _aspalas false)
        (Utilities|FlowControl|DoOnce false) ; enters at Reset
      ))))

(event OnComponentBeginOverlap(Sphere)
  (params (OverlappedComponent :type Primitive%20Component%20Object%20Reference) (OtherActor :type Actor%20Object%20Reference) (OtherComp :type Primitive%20Component%20Object%20Reference) (OtherBodyIndex :type Integer) (bFromSweep :type Boolean) (SweepResult :type Hit%20Result%20Structure%20%28by%20ref%29))
  (if (Utilities|Enum|Equal(Enum) (Utilities|GetObjectName OtherComp) "palas_der")
    (Development|SetHiddeninGame (Variables|Default|Getapuntador) true false)))

(event OnComponentEndOverlap(Sphere)
  (params (OverlappedComponent :type Primitive%20Component%20Object%20Reference) (OtherActor :type Actor%20Object%20Reference) (OtherComp :type Primitive%20Component%20Object%20Reference) (OtherBodyIndex :type Integer))
  (if (Utilities|Enum|Equal(Enum) (Utilities|GetObjectName OtherComp) "palas_der")
    (if (not (Utilities|Enum|Equal(Enum) (Utilities|String|ToString(Text) (Variables|Default|GetHitActor)) "plataforma"))
      (Development|SetHiddeninGame (Variables|Default|Getapuntador) false false))))

(event EventTick
  (params (DeltaSeconds :type Float%20%28single-precision%29))
  (bind _apuntador (Variables|Default|Getapuntador))
  (bind _relativerotation (Variables|/Script/Engine.SceneComponent|GetRelativeRotation _apuntador))
  (bind (_roll _pitch _yaw) (Math|Rotator|BreakRotator _relativerotation))
  (Utilities|FlowControl|Sequence
    (:then_0
      ;[1 1 1] si las palas estan encima de las horquillas al morverse intentara mantener una velocidad linear y angular constante al movimiento del montacragas
      (if (Variables|Default|GetgolpeaPalas)
        (bind _asv_3_3 (Utilities|Casting|CastTov3_3 (Game|Player|GetPlayerPawn 0)))
        (if (Variables|/Game/gus/Monta/blueprints/v3_3/v3_3.v3_3_C|Getesta%20asegurada? _asv_3_3)
          (bind _returnvalue (Physics|GetPhysicsLinearVelocity (Variables|/Game/gus/Monta/blueprints/v3_3/palas.palas_C|Getpalas_base (Variables|/Game/gus/Monta/blueprints/v3_3/v3_3.v3_3_C|Getpalas _asv_3_3)) "None"))
          (Physics|SetPhysicsLinearVelocity (Variables|Debug|GetStaticMeshComponent) (* _returnvalue 1.0) false "None"))))
    (:then_1
      ;[1 1 1] Comment
      (if (Class|Actor|IsActorTickEnabled self)
        (bind _newparam (CallFunction|PointColocar))
        (Variables|Default|SetHitActor _newparam)))
    (:then_2
      (if (Math|Boolean|ANDBoolean (Variables|Default|GetApuntando) (<= (Variables|Default|Getdistancia%20al%20blanco) 8.0) (Utilities|Enum|Equal(Enum) (Utilities|String|ToString(Text) (Variables|Default|GetHitActor)) "plataforma"))
        ;;[1 1 1] sumar +1 o  restar -1 si coloca o no con exito la caja
        (Utilities|FlowControl|DoOnce false :!label _label
          (:Completed
            (bind _asv_3_3_2 (Utilities|Casting|CastTov3_3 (Game|Player|GetPlayerPawn 0)))
            (Variables|Default|SetCaja%20colocada%20con%20Exito true)
            (bind _asplataforma (Utilities|Casting|CastToplataforma (Variables|Default|GetactorGolpeado)))
            (Default|SemaforoAVerde _asplataforma)
            (Default|SumarCajasconExito _asv_3_3_2)
            (goto _label_2 Reset)))
        (else
          (Utilities|FlowControl|DoOnce true :!label _label_2
            (:Completed
              (bind _asv_3_3_3 (Utilities|Casting|CastTov3_3 (Game|Player|GetPlayerPawn 0)))
              (Variables|Default|SetCaja%20colocada%20con%20Exito false)
              (bind _asplataforma_2 (Utilities|Casting|CastToplataforma (Variables|Default|GetactorGolpeado)))
              (Default|SemaforoARojo _asplataforma_2)
              (Default|DecrementarCajascoExito _asv_3_3_3)
              (goto _label Reset))))))
    (:then_3
      ;[1 1 1] rotar apuntador
      (Transformation|SetRelativeRotation _apuntador (Math|Rotator|MakeRotator _roll _pitch (+ _yaw 1.0)) false false))))

(fn ConstructionScript
  (Variables|Default|Settransform%20initial (Transformation|GetWorldTransform (Variables|Debug|GetStaticMeshComponent))))

(fn PointColocar
  (bind _scene (Variables|Default|GetScene))
  (bind _returnvalue (Transformation|GetWorldLocation _scene))
  ;[1 1 1] dibujar laser hacia abajo de la caja, si colisiona con el blanco cambiara de color y aumentara +1 las cajas colocadas, Si no, entonces quitara 1
  (bind _outhit (Collision|LineTraceByChannel _returnvalue (+ _returnvalue (* (* (Math|Vector|GetUpVector _scene) -1.0) 1e+03)) "TraceTypeQuery5" true 0 (select (Variables|Default|GetlaserActivate) "ForOneFrame" "None")))
  (bind _output_get (Variables|Default|Setdistancia%20al%20blanco (.distance _outhit)))
  (bind _output_get_2 (Variables|Default|SetApuntando (.bblockinghit _outhit)))
  (Utilities|FlowControl|Sequence
    (:then_0)
    (:then_1
      (Variables|Default|SetactorGolpeado (.hitactor _outhit))
      (Utilities|IsValid (.hitactor _outhit)
        (:Is%20Valid
          (return (Utilities|Text|ToText(String) (Utilities|String|ToString(Name) (Utilities|Array|Get(acopy) (Variables|/Script/Engine.Actor|GetTags (.hitactor _outhit)))))))))))

(fn Restart
  (Transformation|SetWorldTransform (Variables|Debug|GetStaticMeshComponent) (Variables|Default|Gettransform%20initial) false true))