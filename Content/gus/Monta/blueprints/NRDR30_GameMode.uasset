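; Game mode for a box-placement level with the Monta vehicle, tracking score, boxes and optional time limit.
; Tick updates Monta's metrics widget, while a looping timer runs its box checker.
; Placing all boxes destroys leftover unplaced ones and spawns Parking at the spawner farthest from Monta; losing a box afterwards removes it.
; Expired time or depleted score triggers defeat, destroying Monta and showing the failure screen; Victoria shows completion.
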(event Custom|ComenzarEstacionarse
  ;[1 1 1] Comezar a estacionarse
  (bind _outactors (Actor|GetAllActorsOfClass "/Game/gus/pallet/caja01_BP.caja01_BP_C"))
  (for _array_element _outactors
    (bind _ascaja_01_bp (Utilities|Casting|CastTocaja01_BP _array_element))
    (if (not (Variables|/Game/gus/pallet/caja01_BP.caja01_BP_C|GetCaja%20colocada%20con%20Exito _ascaja_01_bp))
      (Actor|DestroyActor _ascaja_01_bp)))
  (CallFunction|SelectParking))

(event Custom|sumar%20cajas%20con%20exito
  ;[1 1 1] sumar/restar
  (bind _output_get (Variables|Default|Setcajas%20con%20exito (+ (Variables|Default|Getcajas%20con%20exito) 1)))
  (if (== _output_get (Variables|Default|GetCajas%20Totales))
    (Variables|Default|SetFaseDeCajasCompletada? true)
    (CallFunction|ComenzarEstacionarse)
    (else
      (Variables|Default|SetFaseDeCajasCompletada? false))))

(event Custom|decrementar%20cajas%20con%20exito
  ;[1 1 1] sumar/restar
  (Variables|Default|Setcajas%20con%20exito (- (Variables|Default|Getcajas%20con%20exito) 1))
  (if (Variables|Default|GetFaseDeCajasCompletada?)
    (CallFunction|DetenerEstacionarse)))

(event Custom|DetenerEstacionarse
  ;[1 1 1] borra la plataforma de estacionarse
  (bind _outactors (Actor|GetAllActorsOfClass "/Game/gus/environment/parking.parking_C"))
  (for _array_element _outactors
    (Actor|DestroyActor _array_element)))

(event Custom|select%20parking
  ;[1 1 1] select parking y spawnear
  (bind _outactors (Actor|GetAllActorsOfClass "/Game/gus/environment/ParkingSpawner.ParkingSpawner_C"))
  (for _array_element _outactors
    (if (> (Transformation|GetDistanceTo (Variables|Default|Getmonta) _array_element) (Variables|Default|GetdistanciaMax))
      (Variables|Default|SetdistanciaMax (Transformation|GetDistanceTo (Variables|Default|Getmonta) _array_element))
      (Variables|Default|SetparkLocation _array_element)))
  (Game|SpawnActorfromClass "/Game/gus/environment/parking.parking_C" (Transformation|GetWorldTransform (Variables|/Game/gus/environment/ParkingSpawner.ParkingSpawner_C|GetDefaultSceneRoot (Variables|Default|GetparkLocation))) "AlwaysSpawn" 0 (Variables|/Game/gus/environment/ParkingSpawner.ParkingSpawner_C|Getizq/der (Variables|Default|GetparkLocation)) 0)
  (Variables|Default|SetdistanciaMax 0.0))

(event Custom|Spawn%20New%20Parking
  ;[1 1 1] spawnear parkings
  (bind _outactors (Actor|GetAllActorsOfClass "/Game/gus/environment/ParkingSpawner.ParkingSpawner_C"))
  (for _array_element _outactors
    (Game|SpawnActorfromClass "/Game/gus/environment/parking.parking_C" (Transformation|GetWorldTransform (Variables|/Game/gus/environment/ParkingSpawner.ParkingSpawner_C|GetDefaultSceneRoot _array_element)) "Undefined" 0 (Variables|/Game/gus/environment/ParkingSpawner.ParkingSpawner_C|Getizq/der _array_element) 0)))

(event EventBeginPlay
  ;[1 1 1] begin play
  (Utilities|FlowControl|Sequence
    (:then_0
      (bind _asv_3_3 (Utilities|Casting|CastTov3_3 (Game|Player|GetPlayerPawn 0)))
      (Variables|Default|Setmonta _asv_3_3))
    (:then_1
      (Utilities|Time|SetTimerbyFunctionName (Variables|Default|Getmonta) "verificador de cajas" 2.0 true))))

(event EventTick
  (params (DeltaSeconds :type Float%20%28single-precision%29))
  ;[1 1 1] marcar
  (Utilities|IsValid (Variables|Default|Getmonta)
    (:Is%20Valid
      (bind _seg_que_faltan (CallFunction|CalcularTiempo DeltaSeconds))
      (bind _output_get (Variables|Default|Setseg%20que%20faltan _seg_que_faltan))
      (Default|UpdateMetricas (Variables|/Game/gus/Monta/blueprints/v3_3/v3_3.v3_3_C|Getmetri_widget (Variables|Default|Getmonta)) _output_get (Variables|Default|GetIluminacion) (Variables|Default|GetScore) (Variables|Default|GetCajas%20Totales) (Variables|Default|Getcajas%20con%20exito))
      (if (Variables|Default|Getcon%20tiempo?)
        (if (<= _seg_que_faltan 0.0)
          (Utilities|FlowControl|DoOnce false
            (:Completed
              (CallFunction|Derrota))))))))

(event EventCalcularScore
  (params (dañoXgolpe :type Integer))
  ;[1 1 1] calcular score
  (CallFunction|CalcularScore dañoXgolpe))

(fn ConstructionScript)

(fn Victoria
  (bind _returnvalue (Game|GetPlayerController 0))
  (Viewport|RemoveAllWidgets)
  (bind _returnvalue_2 (UserInterface|CreateWidget "/Game/gus/Interfaz/Completado.Completado_C" _returnvalue))
  (bind _output_get (Variables|Default|SetWidget%20completar _returnvalue_2))
  (UserInterface|Viewport|AddtoViewport _output_get 0)
  (Input|SetInputModeUIOnly _returnvalue _output_get "DoNotLock")
  (Variables|/Script/Engine.PlayerController|SetbShowMouseCursor _returnvalue true))

(fn Derrota
  (bind _returnvalue (Game|GetPlayerController 0))
  ;[1 1 1] Derrota - Se ha terminado el tiempo
  (Viewport|RemoveAllWidgets)
  (Pawn|UnPossess _returnvalue)
  (Actor|DestroyActor (Variables|/Game/gus/Monta/blueprints/v3_3/v3_3.v3_3_C|Getpalas (Variables|Default|Getmonta)))
  (bind _returnvalue_2 (UserInterface|CreateWidget "/Game/gus/Interfaz/Fallido.Fallido_C" _returnvalue))
  (bind _output_get (Variables|Default|Setwidget%20gameover _returnvalue_2))
  (UserInterface|Viewport|AddtoViewport _output_get 0)
  (Input|SetInputModeUIOnly _returnvalue _output_get "DoNotLock")
  (Variables|/Script/Engine.PlayerController|SetbShowMouseCursor _returnvalue true))

(fn CalcularTiempo
  (params (delta :type Float%20%28single-precision%29))
  (bind _tiempo_max (Variables|Default|GetTiempo%20Max))
  (if (Variables|Default|Getcon%20tiempo?)
    (bind _output_get (Variables|Default|SetTiempo (+ delta (Variables|Default|GetTiempo))))
    (return (- _tiempo_max _output_get))
    (else
      (return _tiempo_max))))

(fn CalcularScore
  (params (puntos :type Integer))
  (Default|CambiarColorXDaño (Variables|/Game/gus/Monta/blueprints/v3_3/v3_3.v3_3_C|Getmetri_widget (Variables|Default|Getmonta)) puntos)
  (bind _output_get (Variables|Default|SetScore (+ (Variables|Default|GetScore) puntos)))
  (if (<= _output_get 0)
    (CallFunction|Derrota)))