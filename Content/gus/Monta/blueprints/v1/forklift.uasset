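; Forklift vehicle Blueprint that penalizes the player's score for hitting map objects with the forks (Palas).
; Fork hits on anything but a Caja01_BP box apply damage to itself; AnyDamage subtracts it from Score4Win, printing the score or GAME OVER.
; Body (Cuerpo) hits only print a message.
; DoOnce gates with short delays throttle repeat hits, though a box hit never resets the fork gate.
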(event OnComponentHit(palas)
  (params (HitComponent :type Primitive%20Component%20Object%20Reference) (OtherActor :type Actor%20Object%20Reference) (OtherComp :type Primitive%20Component%20Object%20Reference) (NormalImpulse :type Vector :default "0, 0, 0") (Hit :type Hit%20Result%20Structure%20%28by%20ref%29))
  ;[1 1 1] Palas colisionan con objetos
  (Utilities|FlowControl|DoOnce false :!label _label
    (:Completed
      (bind _output_get (Variables|Default|Setactor%20golpeado OtherActor))
      (if (== (Utilities|GetClass _output_get) "/Game/gus/pallet/caja01_BP.caja01_BP_C")
        (Development|PrintText (Utilities|Text|ToText(String) (Utilities|String|Append "Colision: " (Utilities|GetObjectName HitComponent) " - " (Utilities|GetObjectName _output_get))) true true "(R=0.000000,G=1.000000,B=0.241257,A=1.000000)")
        (else
          (Development|PrintText "Golpeaste con las PALAS un objeto del mapa" true true "(R=1.000000,G=0.000000,B=0.071530,A=1.000000)" 0.5)
          (Game|Damage|ApplyDamage self 1e+01 0 0)
          (Utilities|FlowControl|Delay 0.5)
          (goto _label Reset))))))

(event OnComponentHit(cuerpo)
  (params (HitComponent :type Primitive%20Component%20Object%20Reference) (OtherActor :type Actor%20Object%20Reference) (OtherComp :type Primitive%20Component%20Object%20Reference) (NormalImpulse :type Vector :default "0, 0, 0") (Hit :type Hit%20Result%20Structure%20%28by%20ref%29))
  ;[1 1 1] cuerpo golpea con objetos en el mapa
  (Development|PrintText (Utilities|Text|ToText(String) (Utilities|String|Append "Golpeaste con el vehiculo - " (Class|KismetStringLibrary|ToUpper (Class|KismetStringLibrary|ToUpper (Utilities|GetObjectName OtherActor))))) true true "(R=1.000000,G=0.748771,B=0.000000,A=1.000000)"))

(event EventBeginPlay
  (Utilities|FlowControl|Sequence))

(event Game|Damage|EventAnyDamage
  (params (Damage :type Float%20%28single-precision%29) (DamageType :type Damage%20Type%20Object%20Reference) (InstigatedBy :type Controller%20Object%20Reference) (DamageCauser :type Actor%20Object%20Reference))
  ;[1 1 1] Disminuir Score al chocar(PALAS) con objetos que no son palets
  (Utilities|FlowControl|DoOnce false :!label _label
    (:Completed
      (bind _output_get (Variables|Default|SetScore4Win (- (Variables|Default|GetScore4Win) Damage)))
      (if (not (<= _output_get 0.0))
        (Development|PrintText (Utilities|Text|ToText(Float) _output_get "HalfToEven"))
        (Utilities|FlowControl|Delay 0.5)
        (goto _label Reset)
        (else
          (Development|PrintText "GAME OVER" true true "(R=1.000000,G=0.000000,B=0.065193,A=1.000000)" 3.0))))))

(fn ConstructionScript)