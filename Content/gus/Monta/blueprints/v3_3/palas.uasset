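; Forklift fork assembly (palas) for the v3_3 vehicle that senses, carries and releases boxes.
; Each tick, line and box traces find boxes, fade slot markers, set rack up/down locks and, with the bottom-overlap flag, set the loaded state.
; Tick also copies the base's velocity to all parts and moves the PhysicsHandle target that holds secured boxes.
; A damage event reports speed-gated collisions to game-mode scoring with a sound and cooldown.
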(event Custom|asegurar%20caja
  (params (physicHandler :type Physics%20Handle%20Component%20Object%20Reference))
  (bind _handlerlocation1 (Variables|Default|GetHandlerLocation1))
  (bind _caja (Variables|Default|Getcaja))
  ;[1 1 1] Asegurar/liberar caja
  (Utilities|IsValid _caja
    (:Is%20Valid
      (Utilities|FlowControl|DoOnce false
        (:Completed
          (Physics|Components|PhysicsHandle|GrabComponentatLocationwithRotation (Variables|Default|GetPhysicsHandle) (Variables|/Script/Engine.StaticMeshActor|GetStaticMeshComponent _caja) "None" (Transformation|GetWorldLocation _handlerlocation1) (Transformation|GetWorldRotation _handlerlocation1)))))))

(event Custom|liberar%20caja
  (bind _handlerlocation1 (Variables|Default|GetHandlerLocation1))
  (bind _caja (Variables|Default|Getcaja))
  ;[1 1 1] Asegurar/liberar caja
  (Utilities|IsValid _caja
    (:Is%20Valid
      (Physics|Components|PhysicsHandle|ReleaseComponent (Variables|Default|GetPhysicsHandle))
      (Utilities|FlowControl|DoOnce false) ; enters at Reset
    )))

(event Custom|pasar%20daño%20al%20chocar%20con%20entorno
  (params (hit :type Hit%20Result%20Structure) (other%20actor :type Actor%20Object%20Reference))
  (bind _asv_3_3 (Utilities|Casting|CastTov3_3 (Game|Player|GetPlayerPawn 0)))
  (Utilities|FlowControl|DoOnce false :!label _label
    (:Completed
      (if (>= (Math|Float|Floor (Math|Float|Absolute(Float) (* (Class|WheeledVehicleMovementComponent|GetForwardSpeed (Variables|/Script/PhysXVehicles.WheeledVehicle|GetVehicleMovement _asv_3_3)) 0.036))) 5)
        (bind _asnrdr30_game_mode (Utilities|Casting|CastToNRDR30_GameMode (Game|GetGameMode)))
        (Class|InterfaceMetricas|CalcularScore(Message) _asnrdr30_game_mode (Variables|Default|Getdaño))
        (Audio|SpawnSoundatLocation "/Game/gus/Monta/blueprints/NRDR30/sonidos/metal_hit.metal_hit" (.ImpactPoint (Collision|BreakHitResult hit)) "0, 0, 0" 1.0 1.0 0.0 0 0)
        (Utilities|FlowControl|Delay 3.0)
        (goto _label Reset)))))

(event EventTick
  (params (DeltaSeconds :type Float%20%28single-precision%29))
  (bind _laser5 (Variables|Default|Getlaser5))
  (bind _laser4 (Variables|Default|Getlaser4))
  (bind _laser1 (Variables|Default|Getlaser1))
  (bind _laser2 (Variables|Default|Getlaser2))
  (bind _laser3 (Variables|Default|Getlaser3))
  (bind _laser6 (Variables|Default|Getlaser6))
  ;[1 1 1] dibuja los sensores de las palas para saber que objetos se encuentran en rango para ser tomados
  (Utilities|FlowControl|Sequence
    (:then_0
      (CallFunction|DibujarLaser1 _laser1 (Math|Vector|GetForwardVector _laser1) 3e+02))
    (:then_1
      (CallFunction|DibujarLaser2 _laser2 (* (Math|Vector|GetUpVector _laser2) 1.0) 3e+01))
    (:then_2
      (CallFunction|DibujarLaser3 _laser3 (Math|Vector|GetUpVector _laser3) 3e+01))
    (:then_3
      (CallFunction|DibujarLaser4 _laser4 (Math|Vector|GetUpVector _laser4) 1e+01))
    (:then_4
      (CallFunction|DibujarLaser5 _laser5 (Math|Vector|GetUpVector _laser5) 1e+01))
    (:then_5
      (CallFunction|DibujarCajaCentral _laser6 (Math|Vector|GetForwardVector _laser6) 3e+02))
    (:then_6
      (CallFunction|AttachCaja))
    (:then_7
      (CallFunction|StopALLmovement))
    (:then_8
      (CallFunction|AjustarHandlerLocation (Variables|Default|GetPhysicsHandle) (Variables|Default|GetHandlerLocation1)))))

(event Collision|EventHit
  (params (MyComp :type Primitive%20Component%20Object%20Reference) (Other :type Actor%20Object%20Reference) (OtherComp :type Primitive%20Component%20Object%20Reference) (bSelfMoved :type Boolean) (HitLocation :type Vector :default "0, 0, 0") (HitNormal :type Vector :default "0, 0, 0") (NormalImpulse :type Vector :default "0, 0, 0") (Hit :type Hit%20Result%20Structure%20%28by%20ref%29))
  ;[1 1 1] SI golpea con algun objeto, si es diferente de el blueprint de la caja (static mesh) detiene las fisicas
)

(fn ConstructionScript
  (bind _partes_pala (Variables|Default|Getpartes_pala))
  (bind _partes_pala_2 (Variables|Default|Getpartes_pala))
  (bind _partes_postes (Variables|Default|Getpartes_postes))
  ;[0.3899 1 0.3878] Crear arreglos con las partes de la pala
  (Utilities|FlowControl|Sequence
    (:then_0
      (Utilities|Array|Add _partes_postes (Variables|Default|Getposte2))
      (Utilities|Array|Add _partes_postes (Variables|Default|Getposte3))
      (Utilities|Array|Add _partes_postes (Variables|Default|Getposte1))
      (Utilities|Array|Add _partes_pala_2 (Variables|Default|Getdiv_poste1_bloque_chains_030))
      (Utilities|Array|Add _partes_pala_2 (Variables|Default|GetNRDR30_chains_029))
      (Utilities|Array|Add _partes_pala_2 (Variables|Default|GetNRDR30_chains))
      (Utilities|Array|Add _partes_pala_2 (Variables|Default|Getpivote%20union))
      (Utilities|Array|Add _partes_pala_2 (Variables|Default|Getunion))
      (Utilities|Array|Add _partes_pala_2 (Variables|Default|Getunion_tijera1))
      (Utilities|Array|Add _partes_pala_2 (Variables|Default|Getunion_tijera2))
      ;;[1 1 1] SOLO horquillas
      (Utilities|Array|Add _partes_pala (Variables|Default|Getpalas_base))
      (Utilities|Array|Add _partes_pala (Variables|Default|Getpalas_body))
      (Utilities|Array|Add _partes_pala (Variables|Default|Getpalas_der))
      (Utilities|Array|Add _partes_pala (Variables|Default|Getpalas_izq)))
    (:then_1)))

(fn DibujarLaser1
  (params (laser :type Scene%20Component%20Object%20Reference) (vector :type Vector) (distance :type Float%20%28single-precision%29))
  (bind _returnvalue (Transformation|GetWorldLocation laser))
  (bind _outhit (Collision|LineTraceByChannel _returnvalue (+ _returnvalue (* vector distance)) "TraceTypeQuery3" false 0 "None" true "(R=0.000000,G=0.028308,B=0.533333,A=1.000000)" "(R=0.000000,G=1.000000,B=0.000000,A=1.000000)" 1.0))
  (if (.bblockinghit _outhit)
    (Variables|Default|Setlaser1_OK true)
    (bind _ascomponente_de_malla_estática (Utilities|Casting|CastToStaticMeshComponent (.hitcomponent _outhit)))
    (bind _output_get (Variables|Default|SetSlotBox%20mesh _ascomponente_de_malla_estática))
    (bind _returnvalue_2 (Rendering|Material|CreateDynamicMaterialInstance _output_get 0 (Rendering|Material|GetMaterial (.hitcomponent _outhit) 0) "None" :!class /Script/Engine.PrimitiveComponent))
    (bind _output_get_2 (Variables|Default|SetSlotBoxMat2 _returnvalue_2))
    (Rendering|Material|SetScalarParameterValue _output_get_2 "opacidad" (Math|Float|Lerp 0.0 0.15 (Math|Float|NormalizetoRange (.distance _outhit) 1e+01 3e+02)) :!class /Script/Engine.MaterialInstanceDynamic)
    (else
      (Variables|Default|Setlaser1_OK false))))

(fn DibujarLaser2
  (params (laser :type Scene%20Component%20Object%20Reference) (vector :type Vector) (distance :type Float%20%28single-precision%29))
  (bind _returnvalue (Transformation|GetWorldLocation laser))
  (bind _outhit (Collision|LineTraceByChannel _returnvalue (+ _returnvalue (* vector distance)) "TraceTypeQuery5" false 0 "None" true "(R=0.000000,G=0.025643,B=0.533333,A=1.000000)" "(R=0.000000,G=1.000000,B=0.000000,A=1.000000)" 1.0))
  (bind _output_get (Variables|Default|Setlaser2_OK (.bblockinghit _outhit)))
  (if _output_get
    (if (Utilities|Name|Equal(Name) (Utilities|Array|Get(acopy) (Variables|/Script/Engine.ActorComponent|GetComponentTags (.hitcomponent _outhit))) "caja")
      (bind _ascaja_01_bp (Utilities|Casting|CastTocaja01_BP (.hitactor _outhit)))
      (Variables|Default|Setcaja _ascaja_01_bp))))

(fn CheckTocarFondo
  (if (Variables|Default|Getoverlap%20fondo)
    _))

(fn DibujarLaser3
  (params (laser :type Scene%20Component%20Object%20Reference) (vector :type Vector) (distance :type Float%20%28single-precision%29))
  (bind _returnvalue (Transformation|GetWorldLocation laser))
  (bind _outhit (Collision|LineTraceByChannel _returnvalue (+ _returnvalue (* vector distance)) "TraceTypeQuery5" false 0 "None" true "(R=0.004627,G=0.000000,B=0.533333,A=1.000000)" "(R=0.000000,G=1.000000,B=0.000000,A=1.000000)" 1.0))
  (bind _output_get (Variables|Default|Setlaser3_OK (.bblockinghit _outhit)))
  (if _output_get
    _))

(fn AttachCaja
  ;[1 1 1] condicion de que todas las condiciones para tomar caja se han cumplido
  (if (Math|Boolean|ANDBoolean (Variables|Default|Getoverlap%20fondo) (Variables|Default|Getlaser3_OK) (Variables|Default|Getlaser2_OK))
    (Variables|Default|Setcargado true)
    (else
      (Variables|Default|Setcargado false))))

(fn DibujarLaser4
  (params (laser :type Scene%20Component%20Object%20Reference) (vectorUP :type Vector) (distance :type Float%20%28single-precision%29))
  (bind _returnvalue (Transformation|GetWorldRotation laser))
  (bind _returnvalue_2 (Transformation|GetWorldLocation laser))
  (Utilities|FlowControl|Sequence
    (:then_0
      (bind _outhit (Collision|BoxTraceByChannel _returnvalue_2 (+ _returnvalue_2 (* vectorUP distance)) (Variables|Default|Gettam%20vector) _returnvalue "TraceTypeQuery4" false 0 (select (Variables|Default|GetShowLaserUP) "ForOneFrame" "None") true "(R=1.000000,G=0.758785,B=0.000000,A=1.000000)"))
      (Utilities|FlowControl|Sequence
        (:then_0
          (if (.bblockinghit _outhit)
            (if (<= (.distance _outhit) (Variables|Default|GetDistance%20to%20anaquel))
              (Variables|Default|Setlock_up true)
              (else
                (Variables|Default|Setlock_up false :!label _label)))
            (else
              (goto _label))))))
    (:then_1
      (bind _outhit_2 (Collision|BoxTraceByChannel _returnvalue_2 (+ (Transformation|GetWorldLocation laser) (* (* vectorUP -1.0) distance)) (Variables|Default|Gettam%20vector) _returnvalue "TraceTypeQuery4" false 0 (select (Variables|Default|GetShowLaserDown) "ForOneFrame" "None")))
      (if (.bblockinghit _outhit_2)
        (if (<= (.distance _outhit_2) (Variables|Default|GetDistance%20to%20anaquel))
          (Variables|Default|Setlock_down true)
          (else
            (Variables|Default|Setlock_down false :!label _label_2)))
        (else
          (goto _label_2))))))

(fn DibujarCajaCentral
  (params (laser :type Scene%20Component%20Object%20Reference) (vectorUP :type Vector) (distance :type Float%20%28single-precision%29))
  (bind _returnvalue (Transformation|GetWorldLocation laser))
  ;[1 1 1] caja que detecta las cajas
  (Utilities|FlowControl|Sequence
    (:then_0
      (bind _outhit (Collision|BoxTraceByChannel _returnvalue (+ _returnvalue (* vectorUP distance)) "10.000000,50.000000,10.000000" (Transformation|GetWorldRotation laser) "TraceTypeQuery5" false 0 (select (Variables|Default|GetShowLaserCentral) "ForOneFrame" "None") true "(R=0.000000,G=0.371950,B=1.000000,A=1.000000)"))
      (Variables|Default|Setdistancia%20a%20caja (.distance _outhit))
      (if (.bblockinghit _outhit)
        (Variables|Default|Setcaja%20central true)
        (if (and (<= (Variables|Default|Getdistancia%20a%20caja) 1.4e+02) (not (Variables|Default|Getcargado)))
          (bind _asv_3_3 (Utilities|Casting|CastTov3_3 (Game|Player|GetPlayerPawn 0)))
          (elif (<= (Variables|Default|Getdistancia%20a%20caja) 1.4e+02)
            (if (and (<= (Variables|Default|Getdistancia%20a%20caja) 1.4e+02) (Variables|Default|Getcargado))
              (bind _asv_3_3_2 (Utilities|Casting|CastTov3_3 (Game|Player|GetPlayerPawn 0))))))
        (else
          (Variables|Default|Setcaja%20central false))))))

(fn AjustarHandlerLocation
  (params (physicHandle :type Physics%20Handle%20Component%20Object%20Reference) (handlerLocation :type Scene%20Component%20Object%20Reference))
  (Class|PhysicsHandleComponent|SetTargetLocationandRotation physicHandle (Transformation|GetWorldLocation handlerLocation) (Transformation|GetWorldRotation handlerLocation)))

(fn DibujarLaser5
  (params (laser :type Scene%20Component%20Object%20Reference) (vectorUP :type Vector) (distance :type Float%20%28single-precision%29))
  (bind _returnvalue (Transformation|GetWorldRotation laser))
  (bind _returnvalue_2 (Transformation|GetWorldLocation laser))
  ;[1 1 1] Dibuja lasers para horquillas derechas, si golpean con un anaquel, entonces deja de ejercer fuerza hacia arriba o hacia abajo bloqueandose
  (Utilities|FlowControl|Sequence
    (:then_0
      (bind _outhit (Collision|BoxTraceByChannel _returnvalue_2 (+ _returnvalue_2 (* vectorUP distance)) (Variables|Default|Gettam%20vector) _returnvalue "TraceTypeQuery4" false 0 (select (Variables|Default|GetShowLaserUP) "ForOneFrame" "None") true "(R=1.000000,G=0.757948,B=0.000000,A=1.000000)"))
      (if (.bblockinghit _outhit)
        (if (<= (.distance _outhit) (Variables|Default|GetDistance%20to%20anaquel))
          (Variables|Default|Setlock_up2 true)
          (else
            (Variables|Default|Setlock_up2 false :!label _label)))
        (else
          (goto _label))))
    (:then_1
      (bind _outhit_2 (Collision|BoxTraceByChannel _returnvalue_2 (+ (Transformation|GetWorldLocation laser) (* (* vectorUP -1.0) distance)) (Variables|Default|Gettam%20vector) _returnvalue "TraceTypeQuery4" false 0 (select (Variables|Default|GetShowLaserDown) "ForOneFrame" "None")))
      (if (.bblockinghit _outhit_2)
        (if (<= (.distance _outhit_2) (Variables|Default|GetDistance%20to%20anaquel))
          (Variables|Default|Setlock_down2 true)
          (else
            (Variables|Default|Setlock_down2 false :!label _label_2)))
        (else
          (goto _label_2))))))

(fn LiberarInstanciaCaja
  (Actor|Tick|SetActorTickEnabled (Variables|Default|Getcaja)))

(fn StopALLmovement
  (bind _base (Variables|Default|Getbase))
  (bind _returnvalue (Physics|GetPhysicsLinearVelocity _base "None"))
  (Class|PrimitiveComponent|SetAllPhysicsLinearVelocity _base _returnvalue false))

(fn TraceLaserCaja
  (bind _spherecaja (Variables|Default|GetsphereCaja))
  (bind _returnvalue (Transformation|GetWorldLocation _spherecaja))
  (bind (_outhit _returnvalue_2) (Collision|LineTraceForObjects _returnvalue (+ _returnvalue (* (Math|Vector|GetUpVector _spherecaja) 2e+01)) (Utilities|Array|MakeArray "ObjectTypeQuery4") false 0 "Persistent"))
  (return _outhit _returnvalue_2))

(fn Grab
  (params (hit :type Hit%20Result%20Structure))
  (bind _output_get (Variables|Default|Setheld (.HitComponent (Collision|BreakHitResult hit))))
  (Class|PhysicsConstraintComponent|SetConstrainedComponents (Variables|Default|GetgrabConstraint) _output_get "" (Variables|Default|GetsphereCaja) ""))

(fn Release)