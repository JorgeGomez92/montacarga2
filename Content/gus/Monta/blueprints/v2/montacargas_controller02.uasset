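; Player controller for the montacargas02 forklift, turning input into driving, fork control and camera switching.
; On BeginPlay it caches the pawn and its three cameras, which the ChangeCamera action cycles through.
; Drive axes move the pawn forward and yaw it only while forward input is active.
; Fork axes accumulate clamped height, horizontal offset and tilt values without applying them here; the physical animation setup is disconnected.
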(event EventBeginPlay
  (bind _array_cameras (Variables|Default|Getarray_cameras))
  ;[1 1 1] Cambiar de camara 'C'
  (bind _asmontacargas_02 (Utilities|Casting|CastTomontacargas02 (Pawn|GetControlledPawn)))
  (Utilities|FlowControl|Sequence
    (:then_0
      ;;[1 1 1] cargar camaras
      (bind _output_get (Variables|Default|SetmontaC02 _asmontacargas_02))
      (Utilities|Array|Add _array_cameras (Variables|/Game/gus/Monta/blueprints/v2/montacargas02.montacargas02_C|GetCameraMain _output_get))
      (Utilities|Array|Add _array_cameras (Variables|/Game/gus/Monta/blueprints/v2/montacargas02.montacargas02_C|GetCameraMain1 _output_get))
      (Utilities|Array|Add _array_cameras (Variables|/Game/gus/Monta/blueprints/v2/montacargas02.montacargas02_C|GetCameraMain2 _output_get))
      (Variables|Default|SetactualCamera (Variables|/Game/gus/Monta/blueprints/v2/montacargas02.montacargas02_C|GetCameraMain _output_get))
      (Variables|Default|SetnextCamera (Variables|/Game/gus/Monta/blueprints/v2/montacargas02.montacargas02_C|GetCameraMain1 _output_get)))))

(event Input|ActionEvents|InputActionChangeCamera
  (params (Key :type Key%20Structure))
  (bind _array_cameras (Variables|Default|Getarray_cameras))
  (bind _array_cameras_2 (Variables|Default|Getarray_cameras))
  ;[1 1 1] cambiar camara con tecla 'C'
  (:Pressed
    (Components|Activation|Activate (Variables|Default|GetnextCamera) false)
    (Components|Activation|Deactivate (Variables|Default|GetactualCamera))
    (Variables|Default|SetactualCamera (Variables|Default|GetnextCamera))
    (if (== (Utilities|Array|LastIndex _array_cameras_2) (Utilities|Array|FindItem _array_cameras_2 (Variables|Default|GetnextCamera)))
      (Variables|Default|SetnextCamera (Utilities|Array|Get(acopy) (Variables|Default|Getarray_cameras)))
      (else
        (Variables|Default|SetnextCamera (Utilities|Array|Get(acopy) _array_cameras (+ (Utilities|Array|FindItem _array_cameras (Variables|Default|GetnextCamera)) 1)))))))

(event Input|AxisEvents|InputAxisInclinarPalas
  (params (AxisValue :type Float%20%28single-precision%29))
  ;[1 1 1] inclinar palas
  (if (Math|Float|InRange(Float) (Variables|Default|Getinclinacion) -2e+01 2e+01)
    (bind _output_get (Variables|Default|Setinclinacion (+ AxisValue (Variables|Default|Getinclinacion))))
    (if (<= _output_get -2e+01)
      (bind _output_get_2 (Variables|Default|Setinclinacion -2e+01))
      (elif (>= _output_get 2e+01)
        (bind _output_get_3 (Variables|Default|Setinclinacion 2e+01))))))

(event Input|AxisEvents|InputAxisMoveRight
  (params (AxisValue :type Float%20%28single-precision%29))
  ;[1 1 1] input
  (if (!= (Input|AxisValues|GetMoveForward) 0.0)
    (Pawn|Input|AddControllerYawInput (Variables|Default|GetmontaC02) (* AxisValue (Variables|Default|Getvel%20rotacion)))))

(event Input|AxisEvents|InputAxisMoveForward
  (params (AxisValue :type Float%20%28single-precision%29))
  (bind _montac02 (Variables|Default|GetmontaC02))
  ;[1 1 1] input
  (Pawn|Input|AddMovementInput _montac02 (Math|Vector|GetForwardVector (Variables|/Script/Engine.Actor|GetRootComponent _montac02)) (* AxisValue (Variables|Default|Getvel%20mov)) false))

(event Input|AxisEvents|InputAxispalasVertical
  (params (AxisValue :type Float%20%28single-precision%29))
  ;[1 1 1] conseguir alttura
  (if (Math|Float|InRange(Float) (Variables|Default|Getaltura) 0.0 1e+02)
    (bind _output_get (Variables|Default|Setaltura (+ (* AxisValue 0.2) (Variables|Default|Getaltura))))
    (if (<= _output_get 0.0)
      (Variables|Default|Setaltura 0.0)
      (elif (>= _output_get 1e+02)
        (Variables|Default|Setaltura 1e+02)))))

(event Input|AxisEvents|InputAxisPalasHorizontal
  (params (AxisValue :type Float%20%28single-precision%29))
  ;[1 1 1] consehuir valor de palas horizonyal
  (if (Math|Float|InRange(Float) (Variables|Default|Gethorizontal) -5e+01 5e+01)
    (bind _output_get (Variables|Default|Sethorizontal (+ AxisValue (Variables|Default|Gethorizontal))))
    (if (<= _output_get -5e+01)
      (Variables|Default|Sethorizontal -5e+01)
      (elif (>= _output_get 5e+01)
        (Variables|Default|Sethorizontal 5e+01)))))

(fn ConstructionScript)