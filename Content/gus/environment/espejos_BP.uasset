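; Environment mirror prop that reports collision damage to the score when struck by forklift parts.
; A hit on the Lampara component counts if the player's v3_3 vehicle moves at 4 km/h or more and the other actor's second tag is "partemonta".
; It then sends Daño to NRDR30_GameMode, plays a metal sound and permanently reveals a StaticMesh hidden at start.
; A DoOnce with a three-second reset throttles repeat hits.
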(event OnComponentHit(lampara)
  (params (HitComponent :type Primitive%20Component%20Object%20Reference) (OtherActor :type Actor%20Object%20Reference) (OtherComp :type Primitive%20Component%20Object%20Reference) (NormalImpulse :type Vector :default "0, 0, 0") (Hit :type Hit%20Result%20Structure%20%28by%20ref%29))
  ;[1 1 1] Al ser golpeado a una velocidad mayor X y el objeto golpeado sean las palas enviara un mensaje para pasar daño por golpe al score
  (bind _asv_3_3 (Utilities|Casting|CastTov3_3 (Game|Player|GetPlayerPawn 0)))
  (if (and (>= (Math|Float|Floor (Math|Float|Absolute(Float) (* (Class|WheeledVehicleMovementComponent|GetForwardSpeed (Variables|/Script/PhysXVehicles.WheeledVehicle|GetVehicleMovement _asv_3_3)) 0.036))) 4) (Utilities|Name|Equal(Name) (Utilities|Array|Get(acopy) (Variables|/Script/Engine.Actor|GetTags OtherActor) 1) "partemonta"))
    (Utilities|FlowControl|DoOnce false :!label _label
      (:Completed
        (bind _asnrdr30_game_mode (Utilities|Casting|CastToNRDR30_GameMode (Game|GetGameMode)))
        (Class|InterfaceMetricas|CalcularScore(Message) _asnrdr30_game_mode (Variables|Default|Getdaño))
        (Audio|SpawnSoundatLocation "/Game/gus/Monta/blueprints/NRDR30/sonidos/hit_lowmetal.hit_lowmetal" (.ImpactPoint (Collision|BreakHitResult Hit)) "0, 0, 0" 0.7 0.0 0.0 0 0)
        (Rendering|SetVisibility (Variables|Default|GetStaticMesh) true false)
        (Utilities|FlowControl|Delay 3.0)
        (goto _label Reset)))))

(event EventBeginPlay
  (Rendering|SetVisibility (Variables|Default|GetStaticMesh) false false))

(fn ConstructionScript)